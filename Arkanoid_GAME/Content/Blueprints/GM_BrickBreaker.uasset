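; Brick breaker game mode that pre-spawns a small pool of reusable actors: a blocking wall, a test ball and a blocking ball.
; BeginPlay spawns one of each, then parks it hidden with collision and component tick off, zeroing both balls' velocities.
; ActivateFunction moves the pooled wall to the passed-in transform's location and re-enables it, with a debug print.
; Only the wall has activation logic here; the second parameter is unused.
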(event `self.ReceiveBeginPlay`
  ; Pooling
  (bind _returnvalue (`|SpawnActorFromClass` "/Game/Blueprints/BP_BlockingWall.BP_BlockingWall_C" (`KismetMathLibrary.MakeTransform` (0.0 0.0 0.0)) "AlwaysSpawn" "MultiplyWithRoot" null null))
  (bind _output_get (set `self.BlockingWall` _returnvalue))
  (bind _cube (`/Game/Blueprints/BP_BlockingWall.Cube` _output_get))
  (`SceneComponent.SetVisibility` _cube false true)
  (`PrimitiveComponent.SetCollisionEnabled` _cube "NoCollision")
  (`ActorComponent.SetComponentTickEnabled` _cube false)
  (bind _returnvalue_2 (`|SpawnActorFromClass` "/Game/Blueprints/BP_testBall.BP_testBall_C" (`KismetMathLibrary.MakeTransform` (0.0 0.0 0.0)) "AlwaysSpawn" "MultiplyWithRoot" null null))
  (bind _output_get_2 (set `self.TestBall` _returnvalue_2))
  (bind _sphere (`/Game/Blueprints/BP_testBall.Sphere` _output_get_2))
  (`SceneComponent.SetVisibility` _sphere false true)
  (`PrimitiveComponent.SetCollisionEnabled` _sphere "NoCollision")
  (`ActorComponent.SetComponentTickEnabled` _sphere false)
  (set `MovementComponent.Velocity` (0.0 0.0 0.0) (`/Game/Blueprints/BP_testBall.ProjectileMovement` _output_get_2))
  (bind _returnvalue_3 (`|SpawnActorFromClass` "/Game/Blueprints/BP_BlockingBall.BP_BlockingBall_C" (`KismetMathLibrary.MakeTransform` (0.0 0.0 0.0)) "AlwaysSpawn" "MultiplyWithRoot" null null))
  (bind _output_get_3 (set `self.BlockingBall` _returnvalue_3))
  (bind _sphere_2 (`/Game/Blueprints/BP_BlockingBall.Sphere` _output_get_3))
  (`SceneComponent.SetVisibility` _sphere_2 false true)
  (`PrimitiveComponent.SetCollisionEnabled` _sphere_2 "NoCollision")
  (`ActorComponent.SetComponentTickEnabled` _sphere_2 false)
  (set `MovementComponent.Velocity` (0.0 0.0 0.0) (`/Game/Blueprints/BP_BlockingBall.ProjectileMovement` _output_get_3)))

(fn `ActivateFunction`
  (params (NewParam :type "StaticMeshComponent Object Reference") (NewParam1 :type Boolean))
  (bind _returnvalue_location (`KismetMathLibrary.BreakTransform` (`SceneComponent.K2_GetComponentToWorld` NewParam)))
  (`KismetSystemLibrary.PrintString` "Gus")
  (bind _asgm_brick_breaker (cast `/Game/Blueprints/GM_BrickBreaker` (`GameplayStatics.GetGameMode`)))
  (bind _blockingwall (`/Game/Blueprints/GM_BrickBreaker.BlockingWall` _asgm_brick_breaker))
  (`SceneComponent.K2_SetWorldLocationAndRotation` :`self` (`Actor.RootComponent` _blockingwall) :`NewLocation` _returnvalue_location)
  (bind _cube (`/Game/Blueprints/BP_BlockingWall.Cube` _blockingwall))
  (`SceneComponent.SetVisibility` _cube true true)
  (`PrimitiveComponent.SetCollisionEnabled` _cube "QueryAndPhysics")
  (`ActorComponent.SetComponentTickEnabled` _cube true))

(fn `UserConstructionScript`)