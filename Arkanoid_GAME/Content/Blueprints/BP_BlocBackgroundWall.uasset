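; BP_BlocBackgroundWall is a background wall block whose cube changes color according to its Health.
; SetColor compares Health to three exact values and applies the blue, purple or red material instance to the Cube's first slot, from highest to lowest.
; Any other value leaves the material unchanged, and the construction script is empty.
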(fn `SetColor`
  (if (== (`self.health`) 3.0)
    (`PrimitiveComponent.SetMaterial` (`self.Cube`) 0 "/Game/Materials/Blue_instance.Blue_instance")
    (elif (== (`self.health`) 2.0)
      (`PrimitiveComponent.SetMaterial` (`self.Cube`) 0 "/Game/Materials/Purple_instance.Purple_instance")
      (elif (== (`self.health`) 1.0)
        (`PrimitiveComponent.SetMaterial` (`self.Cube`) 0 "/Game/Materials/Red_instance.Red_instance")))))

(fn `UserConstructionScript`)