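; BP_BrickRotation is a destructible brick for a brick-breaker game that loses one Health per BP_testBall hit.
; Its Cube material shows remaining Health (red, purple, blue) and updates after each non-lethal hit.
; Each brick increments NumberOfBricksToDestroy on BP_FPS_Character at BeginPlay and decrements it when destroyed.
; The brick that brings that count to zero calls GM_BrickBreaker's change-level event dispatcher.
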(event `self.ReceiveBeginPlay`
  (`self.SetColor`)
  (bind _asbp_fps_character (cast `/Game/Blueprints/BP_FPS_Character` (`GameplayStatics.GetPlayerCharacter` 0)))
  (set `/Game/Blueprints/BP_FPS_Character.NumberOfBricksToDestroy` (+ (`/Game/Blueprints/BP_FPS_Character.NumberOfBricksToDestroy` _asbp_fps_character) 1) _asbp_fps_character))

(event `self.ReceiveHit`
  (params (MyComp :type "PrimitiveComponent Object Reference") (Other :type "Actor Object Reference") (OtherComp :type "PrimitiveComponent Object Reference") (bSelfMoved :type Boolean) (HitLocation :type "Vector Structure") (HitNormal :type "Vector Structure") (NormalImpulse :type "Vector Structure") (Hit :type "HitResult Structure (by ref)"))
  (cast `/Game/Blueprints/BP_testBall` Other)
  (bind _output_get (set `self.health` (- (`self.health`) 1.0)))
  (if (<= _output_get 0.0)
    (`self.CheckForLevelChange`)
    (`self.K2_DestroyActor`)
    (else
      (`self.SetColor`))))

(fn `CheckForLevelChange`
  (bind _asbp_fps_character (cast `/Game/Blueprints/BP_FPS_Character` (`GameplayStatics.GetPlayerCharacter` 0)))
  (bind _numberofbrickstodestroy (`/Game/Blueprints/BP_FPS_Character.NumberOfBricksToDestroy` _asbp_fps_character))
  (set `/Game/Blueprints/BP_FPS_Character.NumberOfBricksToDestroy` (- _numberofbrickstodestroy 1) _asbp_fps_character)
  (if (<= _numberofbrickstodestroy 0)
    (set `/Game/Blueprints/BP_FPS_Character.NumberOfBricksToDestroy` 0 _asbp_fps_character)
    (bind _asgm_brick_breaker (cast `/Game/Blueprints/GM_BrickBreaker` (`GameplayStatics.GetGameMode`)))
    (`/Game/Blueprints/GM_BrickBreaker.ChangeLevelEventDispatcher` _asgm_brick_breaker)))

(fn `SetColor`
  (if (== (`self.health`) 3.0)
    (`PrimitiveComponent.SetMaterial` (`self.Cube`) 0 "/Game/Materials/Red_instance.Red_instance")
    (elif (== (`self.health`) 2.0)
      (`PrimitiveComponent.SetMaterial` (`self.Cube`) 0 "/Game/Materials/Purple_instance.Purple_instance")
      (elif (== (`self.health`) 1.0)
        (`PrimitiveComponent.SetMaterial` (`self.Cube`) 0 "/Game/Materials/Blue_instance.Blue_instance")))))

(fn `UserConstructionScript`)