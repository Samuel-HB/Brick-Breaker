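; First-person player character for a brick-breaker game, handling Enhanced Input movement, look, shooting and a pause menu.
; Shooting launches the test ball first, then blocking balls until CantShootprojectile resets the cycle, reusing GameMode-held balls by repositioning and re-enabling them.
; Each test shot accrues a penalty that UpdateScore deducts from the bonus saved in GI_Score.
; Forward movement uses a rotated right vector so camera pitch doesn't slow walking.
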(event `self.ReceiveBeginPlay`
  (`self.SetupInput`)
  (bind _asgm_brick_breaker (cast `/Game/Blueprints/GM_BrickBreaker` (`GameplayStatics.GetGameMode`)))
  (add `/Game/Blueprints/GM_BrickBreaker.ChangeLevelEventDispatcher` _asgm_brick_breaker (`|CreateDelegate` :!event `UpdateScore`)))

(event `EnhancedInput|/Game/Input/IA_MoveForward`
  (params (ActionValue :type "Float (double-precision)") (ElapsedSeconds :type "Float (double-precision)") (TriggeredSeconds :type "Float (double-precision)") (InputAction :type "InputAction Object Reference" :default "/Game/Input/IA_MoveForward.IA_MoveForward"))
  (:`Triggered`
    (`self.AddMovementInput` (`KismetMathLibrary.Conv_RotatorToVector` (`KismetMathLibrary.ComposeRotators` (`KismetMathLibrary.Conv_VectorToRotator` (`KismetMathLibrary.GetRightVector` (`self.GetControlRotation`))) (struct :`Yaw` -90.0))) ActionValue)))

(event `EnhancedInput|/Game/Input/IA_MoveRight`
  (params (ActionValue :type "Float (double-precision)") (ElapsedSeconds :type "Float (double-precision)") (TriggeredSeconds :type "Float (double-precision)") (InputAction :type "InputAction Object Reference" :default "/Game/Input/IA_MoveRight.IA_MoveRight"))
  (:`Triggered`
    (`self.AddMovementInput` (`KismetMathLibrary.GetRightVector` (`self.GetControlRotation`)) ActionValue)))

(event `EnhancedInput|/Game/Input/IA_Turn`
  (params (ActionValue :type "Float (double-precision)") (ElapsedSeconds :type "Float (double-precision)") (TriggeredSeconds :type "Float (double-precision)") (InputAction :type "InputAction Object Reference" :default "/Game/Input/IA_Turn.IA_Turn"))
  (:`Triggered`
    (`self.AddControllerYawInput` ActionValue)))

(event `EnhancedInput|/Game/Input/IA_LookUp`
  (params (ActionValue :type "Float (double-precision)") (ElapsedSeconds :type "Float (double-precision)") (TriggeredSeconds :type "Float (double-precision)") (InputAction :type "InputAction Object Reference" :default "/Game/Input/IA_LookUp.IA_LookUp"))
  (:`Triggered`
    (`self.AddControllerPitchInput` ActionValue)))

(event `EnhancedInput|/Game/Input/IA_Shoot`
  (params (ActionValue :type Boolean) (ElapsedSeconds :type "Float (double-precision)") (TriggeredSeconds :type "Float (double-precision)") (InputAction :type "InputAction Object Reference" :default "/Game/Input/IA_Shoot.IA_Shoot"))
  (:`Started`
    (`|PlayMontage` (`self.Mesh`)
      (:`then`
        (if (`self.isFirstShotMade`)
          (`self.ActivateBlockingBall`)
          (bind _asgm_brick_breaker (cast `/Game/Blueprints/GM_BrickBreaker` (`GameplayStatics.GetGameMode`)))
          (`/Game/Blueprints/GM_BrickBreaker.DeactivateBallBarrierEventDispatcher` _asgm_brick_breaker)
          (else
            (`self.ActivateTestBall`)
            (bind _asgm_brick_breaker_2 (cast `/Game/Blueprints/GM_BrickBreaker` (`GameplayStatics.GetGameMode`)))
            (add `/Game/Blueprints/BP_testBall.CantShotprojectileEventDispatcher` (`/Game/Blueprints/GM_BrickBreaker.TestBall` _asgm_brick_breaker_2) (`|CreateDelegate` :!event `CantShootprojectile`))
            (set `self.isFirstShotMade` true)
            (bind _asgm_brick_breaker_3 (cast `/Game/Blueprints/GM_BrickBreaker` (`GameplayStatics.GetGameMode`)))
            (`/Game/Blueprints/GM_BrickBreaker.DeactivateProjectileEventDispatcher` _asgm_brick_breaker_3)
            (set `self.ScorePointsToRemove` (+ (`self.ScorePointsToRemove`) 50))))))))

(event `EnhancedInput|/Game/Input/IA_Jump`
  (params (ActionValue :type Boolean) (ElapsedSeconds :type "Float (double-precision)") (TriggeredSeconds :type "Float (double-precision)") (InputAction :type "InputAction Object Reference" :default "/Game/Input/IA_Jump.IA_Jump"))
  ; Not useful jump
)

(event `EnhancedInput|/Game/Input/IA_Pause`
  (params (ActionValue :type Boolean) (ElapsedSeconds :type "Float (double-precision)") (TriggeredSeconds :type "Float (double-precision)") (InputAction :type "InputAction Object Reference" :default "/Game/Input/IA_Pause.IA_Pause"))
  (:`Started`
    (`self.PauseGame`)))

(fn `ActivateBlockingBall`
  (bind (_returnvalue_location _returnvalue_rotation) (`KismetMathLibrary.BreakTransform` (`SceneComponent.K2_GetComponentToWorld` (`self.ProjectileSpawnLocation`))))
  (bind _asgm_brick_breaker (cast `/Game/Blueprints/GM_BrickBreaker` (`GameplayStatics.GetGameMode`)))
  (bind _blockingball (`/Game/Blueprints/GM_BrickBreaker.BlockingBall` _asgm_brick_breaker))
  (if (not (`SceneComponent.IsVisible` (`/Game/Blueprints/BP_BlockingBall.Sphere` _blockingball)))
    (`SceneComponent.K2_SetWorldLocationAndRotation` (`Actor.RootComponent` _blockingball) _returnvalue_location _returnvalue_rotation false false)
    (bind _sphere (`/Game/Blueprints/BP_BlockingBall.Sphere` _blockingball))
    (`SceneComponent.SetVisibility` _sphere true true)
    (`PrimitiveComponent.SetCollisionEnabled` _sphere "QueryAndPhysics")
    (`ActorComponent.SetComponentTickEnabled` _sphere true)
    (set `MovementComponent.Velocity` (* (`SceneComponent.GetForwardVector` (`self.ProjectileSpawnLocation`)) (`self.BlockingBallVelocity`)) (`/Game/Blueprints/BP_BlockingBall.ProjectileMovement` _blockingball))))

(fn `ActivateTestBall`
  (bind (_returnvalue_location _returnvalue_rotation) (`KismetMathLibrary.BreakTransform` (`SceneComponent.K2_GetComponentToWorld` (`self.ProjectileSpawnLocation`))))
  (bind _asgm_brick_breaker (cast `/Game/Blueprints/GM_BrickBreaker` (`GameplayStatics.GetGameMode`)))
  (bind _testball (`/Game/Blueprints/GM_BrickBreaker.TestBall` _asgm_brick_breaker))
  (`SceneComponent.K2_SetWorldLocationAndRotation` (`Actor.RootComponent` _testball) _returnvalue_location _returnvalue_rotation false false)
  (bind _sphere (`/Game/Blueprints/BP_testBall.Sphere` _testball))
  (`SceneComponent.SetVisibility` _sphere true true)
  (`PrimitiveComponent.SetCollisionEnabled` _sphere "QueryAndPhysics")
  (`ActorComponent.SetComponentTickEnabled` _sphere true)
  (set `MovementComponent.Velocity` (* (`SceneComponent.GetForwardVector` (`self.ProjectileSpawnLocation`)) (`self.ProjectileVelocity`)) (`/Game/Blueprints/BP_testBall.ProjectileMovement` _testball)))

(fn `CantShootprojectile`
  (set `self.isFirstShotMade` false))

(fn `PauseGame`
  (bind _returnvalue (`GameplayStatics.GetPlayerController` 0))
  (if (not (`self.isPauseMenuOpen?`))
    (set `self.isPauseMenuOpen?` true)
    (bind _returnvalue_2 (`|CreateWidget` "/Game/UI/UWB_PauseMenu.UWB_PauseMenu_C" _returnvalue))
    (bind _output_get (set `self.Pause Menu Widget` _returnvalue_2))
    (`UserWidget.AddToViewport` _output_get 0)
    (`WidgetBlueprintLibrary.SetInputMode_GameAndUIEx` _returnvalue (`self.Pause Menu Widget`))
    (set `PlayerController.bShowMouseCursor` true (`GameplayStatics.GetPlayerController` 0))
    (`GameplayStatics.SetGamePaused` true)
    (else
      (set `self.isPauseMenuOpen?` false)
      (`Widget.RemoveFromParent` (`self.Pause Menu Widget`))
      (`GameplayStatics.SetGamePaused` false)
      (`WidgetBlueprintLibrary.SetInputMode_GameOnly` _returnvalue)
      (set `PlayerController.bShowMouseCursor` false (`GameplayStatics.GetPlayerController` 0)))))

(fn `SetupInput`
  (bind _asgi_score (cast `/Game/GI_Score` (`GameplayStatics.GetGameInstance`)))
  (if (`/Game/GI_Score.isGameStarted` _asgi_score)
    (`EnhancedInputSubsystemInterface.AddMappingContext` (pcsubsystem `EnhancedInputLocalPlayerSubsystem` (`GameplayStatics.GetPlayerController` 0)) "/Game/Input/IMC_Player.IMC_Player" 0 (struct))))

(fn `UpdateScore`
  (bind _asgi_score (cast `/Game/GI_Score` (`GameplayStatics.GetGameInstance`)))
  (set `/Game/GI_Score.ScoreSaved` (- (+ (`/Game/GI_Score.ScoreSaved` _asgi_score) 1050) (`self.ScorePointsToRemove`)) _asgi_score)
  (set `self.ScorePointsToRemove` 0)
  (bind _returnvalue (`|CreateWidget` "/Game/UI/UWB_Score.UWB_Score_C" (`GameplayStatics.GetPlayerController` 0)))
  (`UserWidget.AddToViewport` _returnvalue 0))

(fn `UserConstructionScript`)